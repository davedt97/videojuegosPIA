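; Big demon enemy AI that wanders nearby random points until Pawn Sensing spots a MainSWAT, then chases and melees it.
; A recurring timed loop restarts the wander search and clears the seen flag.
; DoOnce gates attack montages, whose notifies apply damage and play impact sound.
; AnyDamage drives health and death, with a montage notify destroying the actor, while Tick updates a camera-facing health bar.
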(event `self.ReceiveBeginPlay`
  (`self.Search around`)
  (`KismetSystemLibrary.Delay` 0.7 :!label _label)
  (`self.Search around`)
  (set `self.HasSeenTarget?` false)
  (goto _label))

(event `Search around`
  ;[0 0 0] Search Around
  (if (not (`self.HasSeenTarget?`))
    (`|AIMoveTo` self (`NavigationSystemV1.K2_GetRandomReachablePointInRadius` (`self.K2_GetActorLocation`) 200.0 null null) null 100.0
      (:`OnSuccess`
        (`KismetSystemLibrary.Delay` 1.0)
        (`self.Search around`)))))

(event `self.ReceiveAnyDamage`
  (params (Damage :type "Float (single-precision)") (DamageType :type "DamageType Object Reference") (InstigatedBy :type "Controller Object Reference") (DamageCauser :type "Actor Object Reference"))
  ;[0 0 0] Health/Damage
  (bind _output_get (set `self.Health` (- (`self.Health`) Damage)))
  (if (<= _output_get 0.0)
    (`KismetSystemLibrary.PrintString` "Dead")
    (`|PlayMontage` (`self.Mesh`) "/Game/Models/BigDemon/ANIM/Dying.Dying"
      (:`then`
        (`CharacterMovementComponent.SetMovementMode` (`self.CharacterMovement`) "MOVE_None" 0)
        (`self.DisableInput` null)
        (set `self.IsDead?` true)
        (`SceneComponent.SetVisibility` (`self.HealthBar`) false false))
      (:`OnNotifyBegin`
        (`self.K2_DestroyActor`)))
    (else
      (`KismetSystemLibrary.PrintString` "Damage"))))

(event `self.PawnSensing.OnSeePawn`
  (params (Pawn :type "Pawn Object Reference"))
  ;[0 0 0] ChasePC
  (bind _asmain_swat (cast `/Game/Models/FINAL_SWAT/MainSWAT` Pawn))
  (`self.ChasePC` Pawn (`/Game/Models/FINAL_SWAT/MainSWAT.Health` _asmain_swat))
  (set `self.hasSeenTarget?` true))

(event `ChasePC`
  (params (TargetActor :type "Actor Object Reference") (A :type "Float (double-precision)"))
  (bind (_returnvalue_x _returnvalue_y) (`KismetMathLibrary.BreakVector` (`self.K2_GetActorLocation` TargetActor)))
  (bind (_returnvalue_x_2 _returnvalue_y_2) (`KismetMathLibrary.BreakVector` (`self.K2_GetActorLocation` self)))
  ;[0 0 0] AttackPC
  (if (not (`self.IsDead?`))
    (`|AIMoveTo` self (0.0 0.0 0.0) TargetActor 150.0
      (:`OnSuccess`
        (`KismetSystemLibrary.PrintString` "Chasing!")
        (if (or (<= (- _returnvalue_x_2 _returnvalue_x) 150.0) (<= (- _returnvalue_y_2 _returnvalue_y) 150.0))
          (`/Engine/EditorBlueprintResources/StandardMacros.DoOnce` false :!label _label_2
            (:`Completed`
              (`Controller.SetControlRotation` (`self.GetController`) (`KismetMathLibrary.FindLookAtRotation` (`self.K2_GetActorLocation`) (`self.K2_GetActorLocation` TargetActor)))
              (`|PlayMontage` (`self.Mesh`) "/Game/Models/BigDemon/ANIM/Attacking_montage.Attacking_montage"
                (:`then`
                  (`KismetSystemLibrary.Delay` 2.0)
                  (if (<= A 0.0)
                    (`CharacterMovementComponent.SetMovementMode` (`self.CharacterMovement`) "MOVE_None" 0)
                    (else
                      (goto _label_2 :!via `Reset`))))
                (:`OnNotifyBegin`
                  (`GameplayStatics.ApplyDamage` TargetActor 25.0)
                  (`GameplayStatics.PlaySoundAtLocation` "/Game/Audio/SWAT/HitImpact_Cue.HitImpact_Cue" (`self.K2_GetActorLocation` self) (struct) 1.0 1.0 0.0 null null null))))))))))

(event `self.ReceiveTick`
  (params (DeltaSeconds :type "Float (single-precision)"))
  ;[0 0 0] EventTick
  (bind _asuw_hud_ai (cast `/Game/HUD/UW_HUD_AI` (`WidgetComponent.GetWidget` (`self.HealthBar`))))
  (`ProgressBar.SetPercent` (`/Game/HUD/UW_HUD_AI.HealthBar` _asuw_hud_ai) (/ (`self.Health`) 100.0))
  (`SceneComponent.K2_SetWorldRotation` (`self.HealthBar`) (`KismetMathLibrary.FindLookAtRotation` (`self.K2_GetActorLocation`) (`PlayerCameraManager.GetCameraLocation` (`GameplayStatics.GetPlayerCameraManager` 0))) false false))

(fn `UserConstructionScript`)